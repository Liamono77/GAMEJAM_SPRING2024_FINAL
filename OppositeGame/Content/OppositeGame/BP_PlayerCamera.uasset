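; Player camera actor that follows its instigating BP_CharacterBase each tick and places its camera on a current target transform.
; On BeginPlay it attaches Target0 to the character's Cambone_0 socket and TargetGame to the GameManager cameraman's message target.
; SetCameraTarget switches targets instantly or starts a timed transform lerp, which UpdateCameraTransform applies every tick.
; It also stores StartRound input and prints debug text; UpdateCombatCamera is an empty stub.
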(event Input|EnhancedActionEvents|EnhancedInputActionIA_StrengthAttack
  (params (ActionValue :type Boolean) (ElapsedSeconds :type Float%20%28double-precision%29) (TriggeredSeconds :type Float%20%28double-precision%29) (InputAction :type Input%20Action%20Object%20Reference :default "/Game/TopDown/Input/Actions/IA_StrengthAttack.IA_StrengthAttack"))
  (:Triggered
    (Development|PrintText "CAMSTRENGTHATTACKLOLOLOL")))

(event Input|EnhancedActionEvents|EnhancedInputActionIA_StartRound
  (params (ActionValue :type Boolean) (ElapsedSeconds :type Float%20%28double-precision%29) (TriggeredSeconds :type Float%20%28double-precision%29) (InputAction :type Input%20Action%20Object%20Reference :default "/Game/TopDown/Input/Actions/IA_StartRound.IA_StartRound"))
  (:Triggered
    (Variables|Default|SetStartRoundInput ActionValue :!label _label))
  (:Started
    (goto _label))
  (:Ongoing
    (goto _label))
  (:Canceled
    (goto _label))
  (:Completed
    (goto _label)))

(event EventBeginPlay
  (bind _returnvalue (Game|GetInstigator))
  (Development|PrintText (Utilities|Text|FormatText "Cam start owner: {s}" (Utilities|GetObjectName _returnvalue)))
  (bind _asbp_character_base (Utilities|Casting|CastToBP_CharacterBase _returnvalue)
    (:then
      (Variables|Default|SetPlayerCharacter _asbp_character_base)
      (CallFunction|BindCameraTargets)
      (CallFunction|SetCameraTarget (Variables|Default|GetTarget0) false 0.0))
    (:CastFailed
      (Development|PrintText "camfailedcast"))))

(event Collision|EventActorBeginOverlap
  (params (OtherActor :type Actor%20Object%20Reference)))

(event EventTick
  (params (DeltaSeconds :type Float%20%28single-precision%29))
  (Utilities|IsValid (Variables|Default|GetPlayerCharacter)
    (:Is%20Valid
      (Transformation|SetActorLocation (Transformation|GetActorLocation (Variables|Default|GetPlayerCharacter)) false false)
      (CallFunction|UpdateCameraTransform))))

(fn ConstructionScript)

(fn SetCameraTarget
  (params (NewTarget :type Static%20Mesh%20Component%20Object%20Reference) (Lerp :type Boolean) (Duration :type Float%20%28double-precision%29) (SenderNameDebug :type Text))
  (Development|PrintText (Utilities|Text|FormatText "CAMERA TARGET SWITCHED, message {m}" SenderNameDebug) true true "(R=1.000000,G=0.000000,B=0.391643,A=1.000000)")
  (if Lerp
    (Variables|Default|SetPrevTarget (Variables|Default|GetCurrentTarget))
    (Variables|Default|SetLerping true)
    (Variables|Default|SetLerpTimer (Utilities|Time|GetTimeSeconds))
    (Variables|Default|SetCurrentTarget NewTarget)
    (Variables|Default|SetLerpDuration Duration)
    (else
      (Variables|Default|SetCurrentTarget NewTarget))))

(fn BindCameraTargets
  (Transformation|AttachComponentToComponent (Variables|Default|GetTarget0) (Variables|/Script/Engine.Character|GetMesh (Variables|Default|GetPlayerCharacter)) "Cambone_0" "KeepRelative" "KeepRelative" "KeepRelative" false)
  (bind _target (Class|BICameraman|GetCameraTarget(Message) (Variables|/Game/OppositeGame/Systems/GameStates/BP_GameManager.BP_GameManager_C|GetCameramanReference (Variables|/Game/OppositeGame/Systems/CharacterEntities/BP_CharacterBase.BP_CharacterBase_C|GetGameManager (Variables|Default|GetPlayerCharacter)))))
  (Transformation|SetWorldTransform (Variables|Default|GetTargetGame) (Transformation|GetWorldTransform _target) false false)
  (Transformation|AttachComponentToComponent (Variables|Default|GetTargetGame) _target "None" "KeepWorld" "KeepWorld" "KeepWorld" true))

(fn UpdateCameraTransform
  (bind _returnvalue (Utilities|Time|GetTimeSeconds))
  (bind _lerptimer (Variables|Default|GetLerpTimer))
  (bind _lerpduration (Variables|Default|GetLerpDuration))
  (bind _returnvalue_2 (- _returnvalue _lerptimer))
  (bind _returnvalue_3 (/ _returnvalue_2 _lerpduration))
  (if (Variables|Default|GetLerping)
    (if (<= _returnvalue_3 1.0)
      (Transformation|SetWorldTransform (Variables|Default|GetCamera) (Math|Transform|Lerp(Transform) (Transformation|GetWorldTransform (Variables|Default|GetPrevTarget)) (Transformation|GetWorldTransform (Variables|Default|GetCurrentTarget)) _returnvalue_3) false false)
      (else
        (Variables|Default|SetLerping false)
        (Transformation|SetWorldTransform (Variables|Default|GetCamera) (Transformation|GetWorldTransform (Variables|Default|GetCurrentTarget)) false false)))
    (else
      (Transformation|SetWorldTransform (Variables|Default|GetCamera) (Transformation|GetWorldTransform (Variables|Default|GetCurrentTarget)) false false))))

(fn UpdateCombatCamera)