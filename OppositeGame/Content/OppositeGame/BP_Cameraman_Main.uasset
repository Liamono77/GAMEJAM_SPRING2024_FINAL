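; BP_Cameraman_Main is a cameraman actor that keeps its TargetGame component aimed at the middle of the active enemies.
; Each tick, after calling the parent Tick, it averages the locations of GameManagerRef.ActiveEnemies.
; It then eases TargetGame's world rotation toward a look-at rotation on that point with RInterpTo, turning in place without moving.
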(event EventBeginPlay
  (|CallParentFunction) ; This node is disabled and will not be called.\nDrag off pins to build functionality.
)

(event Collision|EventActorBeginOverlap
  (params (OtherActor :type Actor%20Object%20Reference))
  (|CallParentFunction OtherActor) ; This node is disabled and will not be called.\nDrag off pins to build functionality.
)

(event EventTick
  (params (DeltaSeconds :type Float%20%28single-precision%29))
  (bind _targetgame (Variables|Default|GetTargetGame))
  (|CallParentFunction DeltaSeconds)
  (bind _returnvalue (Class|GameplayStatics|GetActorArrayAverageLocation (Variables|/Game/OppositeGame/Systems/GameStates/BP_GameManager.BP_GameManager_C|GetActiveEnemies (Variables|Default|GetGameManagerRef))))
  (Transformation|SetWorldRotation (Variables|Default|GetTargetGame) (Math|Interpolation|RInterpTo (Transformation|GetWorldRotation _targetgame) (Math|Rotator|FindLookatRotation (Transformation|GetWorldLocation _targetgame) _returnvalue) DeltaSeconds 5.0) false false))

(fn ConstructionScript
  (|CallParentFunction))