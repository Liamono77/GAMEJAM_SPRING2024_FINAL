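; Targeting helper actor owned by the player's combat state that picks which active enemy is targeted and marks it with a spawned indicator.
; During combat it moves itself from the enemies' average location along the left stick direction, then selects the nearest enemy.
; It retargets immediately on target death, or after a short delay when the stick is pushed or no target exists.
; Otherwise it sits at the indicator.
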(event EventBeginPlay
  (bind _ascst_player_combat (Utilities|Casting|CastToCST_Player_Combat (Components|GetOwner)))
  (Variables|Default|SetController _ascst_player_combat)
  (bind _returnvalue (Game|SpawnActorfromClass "/Game/OppositeGame/Characters/Knight/BP_TargetIndicator.BP_TargetIndicator_C" (Transformation|GetActorTransform) "Undefined" "MultiplyWithRoot" 0 0))
  (Variables|Default|SetTargetIndicator _returnvalue))

(event Collision|EventActorBeginOverlap
  (params (OtherActor :type Actor%20Object%20Reference)))

(event EventTick
  (params (DeltaSeconds :type Float%20%28single-precision%29))
  (bind _closesttarget (Variables|Default|GetClosestTarget))
  (Utilities|IsValid (Variables|Default|GetController)
    (:Is%20Valid
      (Utilities|IsValid _closesttarget
        (:Is%20Valid
          (if (Variables|/Game/OppositeGame/Systems/CharacterEntities/BP_CharacterBase.BP_CharacterBase_C|GetIsDead _closesttarget) ; If dead, get new targ immediately, else do regular process
            (CallFunction|UpdateTarget)
            (else
              (if (or (== (Variables|Default|GetClosestTarget) 0) (> (Math|Vector|VectorLength (Variables|/Game/OppositeGame/Systems/CharacterEntities/CST_Player_Combat.CST_Player_Combat_C|GetLeftStickAxis (Variables|Default|GetController))) 0.5)) :!label _label
                (Utilities|FlowControl|Delay 0.2)
                (CallFunction|UpdateTarget)
                (else
                  (Transformation|SetActorLocation (Transformation|GetActorLocation (Variables|Default|GetTargetIndicator)) false false))))))
        (:Is%20Not%20Valid
          (goto _label))))))

(fn ConstructionScript)

(fn GetClosestTarget
  (for _array_element (Variables|/Game/OppositeGame/Systems/GameStates/BP_GameManager.BP_GameManager_C|GetActiveEnemies (Variables|/Game/OppositeGame/Systems/CharacterEntities/BP_CharacterBase.BP_CharacterBase_C|GetGameManager (Variables|/Game/OppositeGame/Systems/CharacterEntities/CST_CharacterStateTemplate.CST_CharacterStateTemplate_C|GetCharacterRef (Variables|Default|GetController))))
    (if (< (Math|Vector|Distance(Vector) (Transformation|GetActorLocation _array_element) (Transformation|GetActorLocation)) (LocalVariables|GetLowestDist))
      (LocalVariables|SetBestTarget _array_element)
      (LocalVariables|SetLowestDist (Math|Vector|Distance(Vector) (Transformation|GetActorLocation _array_element) (Transformation|GetActorLocation)))))
  (Variables|Default|SetClosestTarget (LocalVariables|GetBestTarget)))

(fn UpdateTarget
  (bind _controller (Variables|Default|GetController))
  (bind _characterref (Variables|/Game/OppositeGame/Systems/CharacterEntities/CST_CharacterStateTemplate.CST_CharacterStateTemplate_C|GetCharacterRef _controller))
  (bind _gamemanager (Variables|/Game/OppositeGame/Systems/CharacterEntities/BP_CharacterBase.BP_CharacterBase_C|GetGameManager _characterref))
  (if (== (Variables|/Game/OppositeGame/Systems/GameStates/BP_GameManager.BP_GameManager_C|GetCurrentState _gamemanager) (Variables|/Game/OppositeGame/Systems/GameStates/BP_GameManager.BP_GameManager_C|GetAC_Combat _gamemanager))
    (bind _returnvalue (Class|GameplayStatics|GetActorArrayAverageLocation (Variables|/Game/OppositeGame/Systems/GameStates/BP_GameManager.BP_GameManager_C|GetActiveEnemies (Variables|/Game/OppositeGame/Systems/CharacterEntities/BP_CharacterBase.BP_CharacterBase_C|GetGameManager (Variables|/Game/OppositeGame/Systems/CharacterEntities/CST_CharacterStateTemplate.CST_CharacterStateTemplate_C|GetCharacterRef (Variables|Default|GetController))))))
    (Transformation|SetActorLocation (+ (* (Math|Vector|Normalize (+ (Variables|/Game/OppositeGame/Systems/CharacterEntities/CST_Player_Combat.CST_Player_Combat_C|GetLeftStickAxis (Variables|Default|GetController)) "0.100000,0.000000,0.000000")) 3e+02) _returnvalue) false false)
    (CallFunction|GetClosestTarget)
    (Transformation|SetActorLocation (Variables|Default|GetTargetIndicator) (Transformation|GetWorldLocation (Variables|/Game/OppositeGame/Systems/CharacterEntities/BP_CharacterBase.BP_CharacterBase_C|GetIndicatorSpawnPosition (Variables|Default|GetClosestTarget))) false false)))