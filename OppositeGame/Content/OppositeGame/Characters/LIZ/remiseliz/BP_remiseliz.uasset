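; BP_remiseliz is a Liz character variant that performs a two-hit strength attack with a remise follow-up against the player.
; It overrides the parent's OVERRIDETHISLOL hook, without calling the parent, to fire the Shiv event.
; Shiv waits EngageDelay, then enqueues two strength-attack actions with different montages, separated by a short delay and targeting the GameManager's player reference.
; A skill-attack step is left unconnected and never runs.
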(event Custom|Shiv
  (bind _gamemanager (Variables|Default|GetGameManager))
  (bind _playerreference (Variables|/Game/OppositeGame/Systems/GameStates/BP_GameManager.BP_GameManager_C|GetPlayerReference _gamemanager))
  (Utilities|FlowControl|Delay (Variables|Default|GetEngageDelay))
  (CallFunction|EnqueueAction "/Game/OppositeGame/Systems/Actions/BP_Action_StrengthAttack.BP_Action_StrengthAttack_C" "/Game/OppositeGame/Characters/LIZ/BaseLiz/Dest/Anims/AS_DualLiz_B_Attack_Strong_A_Montage.AS_DualLiz_B_Attack_Strong_A_Montage" _playerreference)
  (Utilities|FlowControl|Delay 0.75)
  (CallFunction|EnqueueAction "/Game/OppositeGame/Systems/Actions/BP_Action_StrengthAttack.BP_Action_StrengthAttack_C" "/Game/OppositeGame/Characters/LIZ/BaseLiz/Dest/Anims/AS_RemiselisRemise.AS_RemiselisRemise" _playerreference))

(event EventBeginPlay
  (|CallParentFunction) ; This node is disabled and will not be called.\nDrag off pins to build functionality.
)

(event Collision|EventActorBeginOverlap
  (params (OtherActor :type Actor%20Object%20Reference))
  (|CallParentFunction OtherActor) ; This node is disabled and will not be called.\nDrag off pins to build functionality.
)

(event EventTick
  (params (DeltaSeconds :type Float%20%28single-precision%29))
  (|CallParentFunction DeltaSeconds) ; This node is disabled and will not be called.\nDrag off pins to build functionality.
)

(fn ConstructionScript
  (|CallParentFunction))

(fn OVERRIDETHISLOL
  (CallFunction|Shiv))