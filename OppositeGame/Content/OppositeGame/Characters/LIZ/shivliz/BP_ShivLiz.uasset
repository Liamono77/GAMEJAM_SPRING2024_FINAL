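; BP_ShivLiz is a Liz character variant that performs a skill attack against the player.
; It overrides the parent's OVERRIDETHISLOL hook to fire the Shiv event without calling the parent version.
; Shiv waits for EngageDelay, then enqueues a BP_Action_Skill with the base Liz skill montage, targeting the GameManager's player reference.
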(event Custom|Shiv
  (Utilities|FlowControl|Delay (Variables|Default|GetEngageDelay))
  (CallFunction|EnqueueAction "/Game/OppositeGame/Systems/Actions/BP_Action_Skill.BP_Action_Skill_C" "/Game/OppositeGame/Characters/LIZ/shivliz/NewFolder/AS_BaseLiz_Attack_Skill_A_Montage.AS_BaseLiz_Attack_Skill_A_Montage" (Variables|/Game/OppositeGame/Systems/GameStates/BP_GameManager.BP_GameManager_C|GetPlayerReference (Variables|Default|GetGameManager))))

(event EventBeginPlay
  (|CallParentFunction) ; This node is disabled and will not be called.\nDrag off pins to build functionality.
)

(event Collision|EventActorBeginOverlap
  (params (OtherActor :type Actor%20Object%20Reference))
  (|CallParentFunction OtherActor) ; This node is disabled and will not be called.\nDrag off pins to build functionality.
)

(event EventTick
  (params (DeltaSeconds :type Float%20%28single-precision%29))
  (|CallParentFunction DeltaSeconds) ; This node is disabled and will not be called.\nDrag off pins to build functionality.
)

(fn ConstructionScript
  (|CallParentFunction))

(fn OVERRIDETHISLOL
  (CallFunction|Shiv))