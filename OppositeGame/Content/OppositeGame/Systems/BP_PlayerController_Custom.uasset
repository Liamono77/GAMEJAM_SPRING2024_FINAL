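; Custom player controller that sets up Enhanced Input and caches the controlled character.
; On BeginPlay it prints a debug label and, if the input subsystem is valid, adds the default mapping context.
; It then casts the controlled pawn to BP_CharacterBase and stores it as PlayerRef.
; A disconnected leftover chain, which never runs, prints an attack-input message and moves to a fixed location.
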(event Input|EnhancedActionEvents|EnhancedInputActionIA_StrengthAttack
  (params (ActionValue :type Boolean) (ElapsedSeconds :type Float%20%28double-precision%29) (TriggeredSeconds :type Float%20%28double-precision%29) (InputAction :type Input%20Action%20Object%20Reference :default "/Game/TopDown/Input/Actions/IA_StrengthAttack.IA_StrengthAttack")))

(event EventBeginPlay
  (bind _returnvalue (PlayerController|LocalPlayerSubsystems|GetEnhancedInputLocalPlayerSubsystem))
  (Development|PrintText "Player Controller")
  (Utilities|IsValid _returnvalue
    (:Is%20Valid
      (Input|AddMappingContext _returnvalue "/Game/TopDown/Input/IMC_Default.IMC_Default" 0 "(bIgnoreAllPressedKeysUntilRelease=True,bForceImmediately=False)")
      (bind _asbp_character_base (Utilities|Casting|CastToBP_CharacterBase (Pawn|GetControlledPawn)))
      (Variables|Default|SetPlayerRef _asbp_character_base))))

(event EventTick
  (params (DeltaSeconds :type Float%20%28single-precision%29)))

(fn ConstructionScript)