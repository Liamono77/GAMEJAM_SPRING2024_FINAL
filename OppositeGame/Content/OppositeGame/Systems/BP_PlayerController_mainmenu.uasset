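; Main menu player controller, by its name, currently a mostly stubbed input test that prints debug text.
; ManagedStart stores the given player and enables listening, ending in a combat-state cast with no follow-up.
; The strength attack action prints the player's name while listening; StartRound prints a greeting unconditionally.
; BeginPlay is empty, leaving mapping context setup, pawn caching, round-start call and move-to logic disconnected.
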(event Input|EnhancedActionEvents|EnhancedInputActionIA_StrengthAttack
  (params (ActionValue :type Boolean) (ElapsedSeconds :type Float%20%28double-precision%29) (TriggeredSeconds :type Float%20%28double-precision%29) (InputAction :type Input%20Action%20Object%20Reference :default "/Game/TopDown/Input/Actions/IA_StrengthAttack.IA_StrengthAttack"))
  (:Triggered
    (if (Variables|Default|GetListeningForInput)
      (Development|PrintText (Utilities|Text|FormatText "PlayerInput_strangthattack with char {c}" (Utilities|GetObjectName (Variables|Default|GetPlayerRef)))))))

(event Input|EnhancedActionEvents|EnhancedInputActionIA_StartRound
  (params (ActionValue :type Boolean) (ElapsedSeconds :type Float%20%28double-precision%29) (TriggeredSeconds :type Float%20%28double-precision%29) (InputAction :type Input%20Action%20Object%20Reference :default "/Game/TopDown/Input/Actions/IA_StartRound.IA_StartRound"))
  (:Triggered
    (Development|PrintText "Hello")))

(event EventBeginPlay)

(event EventTick
  (params (DeltaSeconds :type Float%20%28single-precision%29)))

(fn ConstructionScript)

(fn ManagedStart
  (params (Player :type BP%20Character%20Base%20Object%20Reference))
  (bind _output_get (Variables|Default|SetPlayerRef Player))
  (Variables|Default|SetListeningForInput true)
  (Utilities|Casting|CastToCST_Player_Combat (Variables|/Game/OppositeGame/Systems/CharacterEntities/BP_CharacterBase.BP_CharacterBase_C|GetCurrentCharacterState _output_get)))