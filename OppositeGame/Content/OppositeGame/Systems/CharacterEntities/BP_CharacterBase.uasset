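; Base character for a queued-action combat system, with debug prints throughout.
; States are spawned, attached actors that possess the character, and the combat state handles offense and some reactions.
; Actions are spawned actors added to shared and offense/defense queues; Tick pops the shared queue whenever CurrentAction matches one specific value.
; Incoming attacks turn the character toward the aggressor and play hurt or block montages, while helpers spawn indicator effects by action type.
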(event EventBeginPlay
  (bind _asbp_game_manager (Utilities|Casting|CastToBP_GameManager (Components|GetOwner)))
  (Development|PrintText (Utilities|Text|FormatText "game manager: {g}, msg: {s}" (Utilities|GetObjectName _asbp_game_manager) (Variables|/Game/OppositeGame/Systems/GameStates/BP_GameManager.BP_GameManager_C|GetTestVar _asbp_game_manager)))
  (Variables|Default|SetGameManager _asbp_game_manager))

(event Collision|EventActorBeginOverlap
  (params (OtherActor :type Actor%20Object%20Reference)))

(event EventTick
  (params (DeltaSeconds :type Float%20%28single-precision%29))
  (if (Utilities|Enum|Equal(Enum) (Variables|Default|GetCurrentAction) "NewEnumerator4")
    (CallFunction|DequeueAction)))

(fn ConstructionScript)

(fn EngageOffense
  (Development|PrintText (Utilities|Text|FormatText "Character {c} is taking an offense action" (Utilities|GetObjectName self)))
  (Default|EngageOffense (Variables|Default|GetCombatStateRef)))

(fn SwitchtoState
  (params (StateToLoad :type CST%20Character%20State%20Template%20Class%20Reference))
  (bind _self self)
  (Development|PrintText (Utilities|Text|FormatText "Character {C} is switching to state {s}" (Utilities|GetObjectName self) (Utilities|GetClassDisplayName StateToLoad)))
  (Utilities|IsValid (Variables|Default|GetCurrentCharacterState)
    (:Is%20Valid
      (Actor|DestroyActor (Variables|Default|GetCurrentCharacterState)))
    (:Is%20Not%20Valid
      _))
  (bind _returnvalue (Game|SpawnActorfromClass StateToLoad (Transformation|GetActorTransform) "Undefined" "MultiplyWithRoot" _self _self))
  (Pawn|Possess _returnvalue self)
  (Transformation|AttachActorToActor _returnvalue self "None" "KeepWorld" "KeepWorld" "KeepWorld" true)
  (Variables|Default|SetCurrentCharacterState _returnvalue)
  (if (== StateToLoad (Variables|Default|GetCombatStateToLoad))
    (bind _ascst_combat_base (Utilities|Casting|CastToCST_Combat_Base _returnvalue))
    (bind _output_get (Variables|Default|SetCombatStateRef _ascst_combat_base))
    (Development|PrintText "COMBATSTATESET" true true "(R=0.157399,G=1.000000,B=0.000000,A=1.000000)")
    (Default|TestFunction _output_get)))

(fn PlayCinematicMontage
  (params (Montage :type Anim%20Montage%20Object%20Reference))
  (bind _returnvalue (Animation|Montage|MontagePlay (Components|SkeletalMesh|GetAnimInstance (Variables|Character|GetMesh)) Montage 1.0 "MontageLength" 0.0 true))
  (return _returnvalue))

(fn InitializeRefs
  (params (Manager :type BP%20Game%20Manager%20Object%20Reference) (Target :type BP%20Character%20Base%20Object%20Reference))
  (bind _output_get (Variables|Default|SetGameManager Manager))
  (Variables|Default|SetCombatStartTargetPosition (* (Math|Vector|Normalize (- (Transformation|GetActorLocation) (Transformation|GetActorLocation _output_get))) (Variables|/Game/OppositeGame/Systems/GameStates/BP_GameManager.BP_GameManager_C|GetDesiredEnemyDistance (Variables|Default|GetGameManager))))
  (Variables|Default|SetCurrentTarget Target))

(fn SpawnEffect
  (params (IndicatorToSpawn :type BP%20Indicator%20Base%20Class%20Reference) (ActionType :type ActionType%20Enum :default "NewEnumerator0"))
  (if (Utilities|Enum|Equal(Enum) ActionType "NewEnumerator4")
    (CallFunction|SpawnEffectB "/Game/OppositeGame/Systems/Idic/BP_IndicatorBase.BP_IndicatorBase_C")
    (elif (Utilities|Enum|Equal(Enum) ActionType "NewEnumerator0")
      (CallFunction|SpawnEffectB "/Game/OppositeGame/Systems/Idic/BP_Indicator_Strong.BP_Indicator_Strong_C")
      (elif (Utilities|Enum|Equal(Enum) ActionType "NewEnumerator1")
        (CallFunction|SpawnEffectB "/Game/OppositeGame/Systems/Idic/BP_Indicator_Skill.BP_Indicator_Skill_C")
        (elif (Utilities|Enum|Equal(Enum) ActionType "NewEnumerator2")
          (CallFunction|SpawnEffectB "/Game/OppositeGame/Systems/Idic/BP_Indicator_Dodge.BP_Indicator_Dodge_C")
          (elif (Utilities|Enum|Equal(Enum) ActionType "NewEnumerator3")
            (CallFunction|SpawnEffectB "/Game/OppositeGame/Systems/Idic/BP_Indicator_Block.BP_Indicator_Block_C")))))))

(fn SpawnEffectB
  (params (NewParam :type BP%20Indicator%20Base%20Class%20Reference))
  (bind _returnvalue (Game|SpawnActorfromClass NewParam (Transformation|GetWorldTransform (Variables|Default|GetIndicatorSpawnPosition)) "Undefined" "MultiplyWithRoot" 0 self))
  (Transformation|AddActorWorldOffset _returnvalue (* (Math|Random|RandomUnitVector) 25.0))
  (Transformation|AttachComponentToComponent _returnvalue (Variables|Default|GetIndicatorSpawnPosition) "None" "KeepWorld" "KeepWorld" "KeepWorld" true))

(fn DodgedAnAttack
  (params (Aggressor :type BP%20Character%20Base%20Object%20Reference) (HitDirection :type Integer))
  (Development|PrintText (Utilities|Text|FormatText "Character {c} dodged an attack from character {A}" (Utilities|GetObjectName self) (Utilities|GetObjectName Aggressor))))

(fn BlockedAnAttack
  (params (Aggressor :type BP%20Character%20Base%20Object%20Reference) (HitDirection :type Integer))
  (Development|PrintText (Utilities|Text|FormatText "Character {c} blocked an attack from character {A}" (Utilities|GetObjectName self) (Utilities|GetObjectName Aggressor))))

(fn HitbyAnAttack
  (params (Aggressor :type BP%20Character%20Base%20Object%20Reference) (HitDirection :type Integer))
  (bind _mesh (Variables|Character|GetMesh))
  (bind _montageshurt (Variables|Default|GetMontagesHurt))
  (bind _returnvalue (Components|SkeletalMesh|GetAnimInstance _mesh))
  (bind _output (Utilities|Array|Get(acopy) _montageshurt HitDirection))
  (CallFunction|IncomingAttack Aggressor HitDirection)
  (Development|PrintText (Utilities|Text|FormatText "Character {c} Was hit by an attack from character {A}" (Utilities|GetObjectName self) (Utilities|GetObjectName Aggressor)))
  (Utilities|IsValid _output
    (:Is%20Valid
      (Animation|Montage|MontagePlay _returnvalue _output 1.0 "MontageLength" 0.0 true))
    (:Is%20Not%20Valid
      (Animation|Montage|MontagePlay _returnvalue (Utilities|Array|Get(acopy) (Variables|Default|GetMontagesHurt)) 1.0 "MontageLength" 0.0 true))))

(fn IncomingAttack
  (params (Aggressor :type BP%20Character%20Base%20Object%20Reference) (HitDirection :type Integer))
  (Transformation|SetActorRotation (Math|Rotator|FindLookatRotation (Transformation|GetActorLocation) (Transformation|GetActorLocation Aggressor))))

(fn ProcessIncomingAttackUniv
  (params (Aggressor :type BP%20Character%20Base%20Object%20Reference) (HitDirection :type Integer) (MontageSet :type Array%20of%20Anim%20Montage%20Object%20References) (ShouldHurt :type Boolean) (ReactionType :type ReactionType%20Enum :default "NewEnumerator0"))
  (bind _returnvalue (Math|Random|RandomIntegerinRange 0 2))
  (bind _mesh (Variables|Character|GetMesh))
  (bind _returnvalue_2 (Components|SkeletalMesh|GetAnimInstance _mesh))
  (bind _output (Utilities|Array|Get(acopy) MontageSet _returnvalue))
  (Utilities|FlowControl|Sequence
    (:then_0
      (CallFunction|IncomingAttack Aggressor HitDirection)
      (Development|PrintText (Utilities|Text|FormatText "Character {c} Was targeted by an attack from character {A}" (Utilities|GetObjectName self) (Utilities|GetObjectName Aggressor)))
      (Utilities|IsValid _output
        (:Is%20Valid
          (Animation|Montage|MontagePlay _returnvalue_2 _output 1.0 "MontageLength" 0.0 true))
        (:Is%20Not%20Valid
          (Animation|Montage|MontagePlay _returnvalue_2 (Utilities|Array|Get(acopy) MontageSet) 1.0 "MontageLength" 0.0 true))))
    (:then_1
      (if ShouldHurt
        (CallFunction|HurtFunctionality Aggressor)))))

(fn HurtFunctionality
  (params (Aggressor :type BP%20Character%20Base%20Object%20Reference))
  (Development|PrintText (Utilities|Text|FormatText "Character {c} Was hit by an attack from character {A}" (Utilities|GetObjectName self) (Utilities|GetObjectName Aggressor))))

(fn ProcessIncomingAttackUnivB
  (params (Aggressor :type BP%20Character%20Base%20Object%20Reference) (HitDirection :type Integer) (ReactionType :type ReactionType%20Enum :default "NewEnumerator0"))
  (bind _returnvalue (Math|Random|RandomIntegerinRange 0 2))
  (bind _mesh (Variables|Character|GetMesh))
  (bind _montageshurt (Variables|Default|GetMontagesHurt))
  (bind _montagesblock (Variables|Default|GetMontagesBlock))
  (bind _mesh_2 (Variables|Character|GetMesh))
  (bind _returnvalue_2 (Components|SkeletalMesh|GetAnimInstance _mesh_2))
  (bind _returnvalue_3 (Components|SkeletalMesh|GetAnimInstance _mesh))
  (bind _output (Utilities|Array|Get(acopy) _montageshurt HitDirection))
  (bind _output_2 (Utilities|Array|Get(acopy) _montagesblock _returnvalue))
  (Development|PrintText (Utilities|Text|FormatText "Character {c} Was targeted by an attack from character {A}, reaction type {r}" (Utilities|GetObjectName self) (Utilities|GetObjectName Aggressor) (Utilities|String|EnumtoString ReactionType)))
  (CallFunction|IncomingAttack Aggressor HitDirection)
  (if (Utilities|Enum|Equal(Enum) ReactionType "NewEnumerator0")
    (Utilities|IsValid _output
      (:Is%20Valid
        (Animation|Montage|MontagePlay _returnvalue_3 _output 1.0 "MontageLength" 0.0 true))
      (:Is%20Not%20Valid
        (Animation|Montage|MontagePlay _returnvalue_3 (Utilities|Array|Get(acopy) _montageshurt) 1.0 "MontageLength" 0.0 true)))
    (CallFunction|SetCurrentAction "NewEnumerator5" "WasHurt")
    (elif (Utilities|Enum|Equal(Enum) ReactionType "NewEnumerator1")
      (Utilities|IsValid _output_2
        (:Is%20Valid
          (Animation|Montage|MontagePlay _returnvalue_2 _output_2 1.0 "MontageLength" 0.0 true))
        (:Is%20Not%20Valid
          (Animation|Montage|MontagePlay _returnvalue_2 (Utilities|Array|Get(acopy) _montagesblock) 1.0 "MontageLength" 0.0 true)))
      (elif (Utilities|Enum|Equal(Enum) ReactionType "NewEnumerator2")
        (Default|ProcessReaction (Variables|Default|GetCombatStateRef) Aggressor HitDirection ReactionType)))))

(fn EnqueueAction
  (params (Action :type BP%20Action%20Base%20Class%20Reference) (MontageToPlay :type Anim%20Montage%20Object%20Reference) (TargetedCharacter :type BP%20Character%20Base%20Object%20Reference))
  (bind _self self)
  (Development|PrintText (Utilities|Text|FormatText "Character {c} is enqueueing an action: {a}" (Utilities|GetObjectName self) (Utilities|GetClassDisplayName Action)) true true "(R=1.000000,G=0.890440,B=0.251666,A=1.000000)" 3.0)
  (bind _returnvalue (Game|SpawnActorfromClass Action (Transformation|GetActorTransform _self) "Undefined" "MultiplyWithRoot" 0 _self))
  (Transformation|AttachActorToActor _returnvalue self "None" "KeepWorld" "KeepWorld" "KeepWorld" false)
  (Default|GetActionTarget (Variables|Default|GetCombatStateRef))
  (Default|Initialize _returnvalue self TargetedCharacter MontageToPlay)
  (Utilities|Array|Add (Variables|Default|GetActionQueueShared) _returnvalue)
  (if (or (Utilities|Enum|Equal(Enum) (Variables|/Game/OppositeGame/Systems/Actions/BP_ActionBase.BP_ActionBase_C|GetActionType _returnvalue) "NewEnumerator0") (Utilities|Enum|Equal(Enum) (Variables|/Game/OppositeGame/Systems/Actions/BP_ActionBase.BP_ActionBase_C|GetActionType _returnvalue) "NewEnumerator1"))
    (Utilities|Array|Add (Variables|Default|GetActionQueueOffense) _returnvalue)
    (elif (or (Utilities|Enum|Equal(Enum) (Variables|/Game/OppositeGame/Systems/Actions/BP_ActionBase.BP_ActionBase_C|GetActionType _returnvalue) "NewEnumerator2") (Utilities|Enum|Equal(Enum) (Variables|/Game/OppositeGame/Systems/Actions/BP_ActionBase.BP_ActionBase_C|GetActionType _returnvalue) "NewEnumerator3"))
      (Utilities|Array|Add (Variables|Default|GetActionQueueDefense) _returnvalue))))

(fn DequeueAction
  (bind _actionqueueshared (Variables|Default|GetActionQueueShared))
  (bind _output (Utilities|Array|Get(acopy) _actionqueueshared))
  (Utilities|IsValid _output
    (:Is%20Valid
      (Default|Pop _output)
      (Variables|Default|SetCurrentAction (Variables|/Game/OppositeGame/Systems/Actions/BP_ActionBase.BP_ActionBase_C|GetActionType _output))
      (Utilities|Array|RemoveIndex _actionqueueshared))))

(fn SetCurrentAction
  (params (ActionType :type ActionType%20Enum :default "NewEnumerator4") (Explanation :type Text))
  (Development|PrintText (Utilities|Text|FormatText "Character {c} had its current action state set to {x}, explanation: {e}" (Utilities|GetObjectName self) (Utilities|String|EnumtoString ActionType) Explanation) true true "(R=1.000000,G=0.971056,B=0.260197,A=1.000000)" 3.0)
  (Variables|Default|SetCurrentAction ActionType)
  (Default|SetCurrentActionOverrideable (Variables|Default|GetCombatStateRef) ActionType Explanation))