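; BP_ActionBase is a base Blueprint for character actions, pairing an effect with an animation montage.
; Initialize stores the acting character, target character and montage, and immediately has the acting character spawn an effect for this action's type.
; Pop later plays the stored montage on the acting character's mesh anim instance.
; The stored target is unused here, and the event graph and construction script are empty.
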(event EventBeginPlay)

(event Collision|EventActorBeginOverlap
  (params (OtherActor :type Actor%20Object%20Reference)))

(event EventTick
  (params (DeltaSeconds :type Float%20%28single-precision%29)))

(fn ConstructionScript)

(fn Initialize
  (params (CharacterReference :type BP%20Character%20Base%20Object%20Reference) (TargetCharacter :type BP%20Character%20Base%20Object%20Reference) (MontageToPlay :type Anim%20Montage%20Object%20Reference))
  (bind _output_get (Variables|Default|SetCharacterRef CharacterReference))
  (Default|SpawnEffect _output_get 0 (Variables|Default|GetActionType))
  (Variables|Default|SetTargetCharacter TargetCharacter)
  (Variables|Default|SetMontageToPlay MontageToPlay))

(fn Pop
  (Animation|Montage|MontagePlay (Components|SkeletalMesh|GetAnimInstance (Variables|/Script/Engine.Character|GetMesh (Variables|Default|GetCharacterRef))) (Variables|Default|GetMontageToPlay) 1.0 "MontageLength" 0.0 true))