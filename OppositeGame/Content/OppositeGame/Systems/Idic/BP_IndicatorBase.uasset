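; BP_IndicatorBase is a short-lived visual indicator that pops in with a sound and removes itself after one second.
; On BeginPlay it creates a dynamic material, spawns an attached BP_IndicatorBackround tinted with ColorDesired, and sets its lifespan.
; Tick copies the player camera's rotation, quickly scales the actor up to full size, and drives the material's LerpValue with a parabolic curve over elapsed time.
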(event EventBeginPlay
  (bind _staticmesh1 (Variables|Default|GetStaticMesh1))
  (CallFunction|CreateMatInstance)
  (bind _returnvalue (Game|SpawnActorfromClass "/Game/OppositeGame/Systems/Idic/BP_IndicatorBackround.BP_IndicatorBackround_C" (Transformation|GetWorldTransform _staticmesh1) "Undefined" "MultiplyWithRoot" 0 0))
  (Transformation|AttachComponentToComponent _returnvalue _staticmesh1 "None" "KeepWorld" "KeepWorld" "KeepWorld" true)
  (Default|CreateMatInstance _returnvalue (Variables|Default|GetColorDesired))
  (Audio|SpawnSoundatLocation (Variables|Default|GetSoundFX) (Transformation|GetActorLocation) "0, 0, 0" 0.3 2.0 0.0 0 0)
  (Actor|SetLifeSpan 1.0))

(event Collision|EventActorBeginOverlap
  (params (OtherActor :type Actor%20Object%20Reference)))

(event EventTick
  (params (DeltaSeconds :type Float%20%28single-precision%29))
  (bind _output_get (Variables|Default|SetMyTimer (+ (Variables|Default|GetMyTimer) DeltaSeconds)))
  (CallFunction|SetIntensity _output_get)
  (Transformation|SetActorTransform (Math|Transform|MakeTransform (.location (Transformation|GetActorTransform)) (Camera|GetCameraRotation (Game|GetPlayerCameraManager 0)) (* (Math|Float|Clamp(Float) (* _output_get 1e+01)) "1.000000,1.000000,1.000000")))
  (Rendering|Material|SetScalarParameterValue (Variables|Default|GetMaterialInstance) "LerpValue" (Variables|Default|GetIntensityValue) :!class /Script/Engine.MaterialInstanceDynamic))

(fn ConstructionScript)

(fn CreateMatInstance
  (bind _returnvalue (Rendering|Material|CreateDynamicMaterialInstance (Variables|Default|GetStaticMesh) 0 0 "None" :!class /Script/Engine.PrimitiveComponent))
  (Variables|Default|SetMaterialInstance _returnvalue))

(fn SetIntensity
  (params (LinearThing :type Float%20%28double-precision%29))
  (Variables|Default|SetIntensityValue (* (+ (* LinearThing (* LinearThing -2.0)) LinearThing) 4.0)))