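; Short-lived indicator background actor that faces the player camera, grows, and destroys itself after one second.
; Tick accumulates a timer that drives linear scale growth and a quadratic intensity curve written to the material's LerpValue.
; CreateMatInstance builds the colored dynamic material but has no live call in this Blueprint.
; SetColor is empty, and several leftover debug and test chains are disconnected.
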(event EventBeginPlay
  (Actor|SetLifeSpan 1.0))

(event Collision|EventActorBeginOverlap
  (params (OtherActor :type Actor%20Object%20Reference)))

(event EventTick
  (params (DeltaSeconds :type Float%20%28single-precision%29))
  (bind _output_get (Variables|Default|SetMyTimer (+ (Variables|Default|GetMyTimer) DeltaSeconds)))
  (CallFunction|SetIntensity _output_get)
  (Transformation|SetActorTransform (Math|Transform|MakeTransform (.location (Transformation|GetActorTransform)) (Camera|GetCameraRotation (Game|GetPlayerCameraManager 0)) (* (* _output_get 1e+01) "1.000000,1.000000,1.000000")))
  (Rendering|Material|SetScalarParameterValue (Variables|Default|GetMaterialInstance) "LerpValue" (Variables|Default|GetIntensityValue) :!class /Script/Engine.MaterialInstanceDynamic))

(fn ConstructionScript)

(fn CreateMatInstance
  (params (ColorDesired :type Color%20Structure))
  (bind _returnvalue (Rendering|Material|CreateDynamicMaterialInstance (Variables|Default|GetStaticMesh) 0 0 "None" :!class /Script/Engine.PrimitiveComponent))
  (Variables|Default|SetMaterialInstance _returnvalue)
  (Rendering|Material|SetVectorParameterValue _returnvalue "Color" (Math|Conversions|ToLinearColor(Color) ColorDesired) :!class /Script/Engine.MaterialInstanceDynamic))

(fn SetIntensity
  (params (LinearThing :type Float%20%28double-precision%29))
  (Variables|Default|SetIntensityValue (* (+ (* LinearThing (* LinearThing -5.0)) LinearThing) 8.0)))

(fn SetColor)