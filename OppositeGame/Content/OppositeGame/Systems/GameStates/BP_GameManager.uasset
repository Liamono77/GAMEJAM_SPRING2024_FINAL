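; BP_GameManager is the game's central manager, setting up the player, cameras and enemies and running the game's state machine.
; On BeginPlay it spawns the player, cameraman and player camera, then registers every other placed BP_CharacterBase as an active enemy targeting the player.
; It starts in the ACCombat state, with SwitchToState calling exit and enter hooks and Tick forwarding updates to the current state.
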(event EventBeginPlay
  (Utilities|FlowControl|Sequence
    (:then_0
      (bind _returnvalue (Game|SpawnActorfromClass "/Game/OppositeGame/Systems/CharacterEntities/BP_Char_Player.BP_Char_Player_C" (Transformation|GetActorTransform) "Undefined" "MultiplyWithRoot" 0 0))
      (Default|InitializeRefs _returnvalue self)
      (bind _output_get (Variables|Default|SetPlayerReference _returnvalue))
      (bind _returnvalue_2 (Game|SpawnActorfromClass (Variables|Default|GetCameraman) (Transformation|GetActorTransform (Variables|Default|GetPlayerReference)) "Undefined" "MultiplyWithRoot" self 0))
      (Variables|Default|SetCameramanReference _returnvalue_2)
      (bind _returnvalue_3 (Game|SpawnActorfromClass "/Game/OppositeGame/BP_PlayerCamera.BP_PlayerCamera_C" (Transformation|GetActorTransform _output_get) "Undefined" "MultiplyWithRoot" 0 _output_get))
      (Variables|Default|SetPlayerCamReference _returnvalue_3))
    (:then_1
      (CallFunction|InitializeEnemies))
    (:then_2
      (CallFunction|SwitchtoState (Variables|Default|GetAC_Combat)))))

(event Collision|EventActorBeginOverlap
  (params (OtherActor :type Actor%20Object%20Reference)))

(event EventTick
  (params (DeltaSeconds :type Float%20%28single-precision%29))
  (bind _currentstate (Variables|Default|GetCurrentState))
  (Utilities|IsValid _currentstate
    (:Is%20Valid
      (Default|OnStateUpdate _currentstate DeltaSeconds))))

(fn ConstructionScript)

(fn SwitchtoState
  (params (NextState :type AC%20Game%20State%20Template%20Object%20Reference))
  (Development|PrintText (Utilities|Text|FormatText "GAMEMANAGER: Switching to state {S}" (Utilities|GetObjectName NextState)))
  (Utilities|IsValid (Variables|Default|GetCurrentState)
    (:Is%20Valid
      (Default|OnStateExit (Variables|Default|GetCurrentState)))
    (:Is%20Not%20Valid
      _))
  (bind _output_get (Variables|Default|SetCurrentState NextState))
  (Default|OnStateEnter _output_get))

(fn InitializeEnemies
  (bind _outactors (Actor|GetAllActorsOfClass "/Game/OppositeGame/Systems/CharacterEntities/BP_CharacterBase.BP_CharacterBase_C"))
  (Development|PrintText (Utilities|Text|FormatText "Checking {x} enemies..." (Utilities|Array|Length _outactors)))
  (for (_array_element _array_index) _outactors
    (if (!= _array_element (Variables|Default|GetPlayerReference))
      (Default|InitializeRefs _array_element self (Variables|Default|GetPlayerReference))
      (Utilities|Array|Add (Variables|Default|GetActiveEnemies) _array_element)
      (Development|PrintText (Utilities|Text|FormatText "Char in slot {a}: {b}" _array_index (Utilities|GetDisplayName _array_element))))))