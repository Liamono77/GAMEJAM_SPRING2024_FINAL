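; Game manager state for active combat, which paces enemy attacks and decides when the fight ends.
; On enter it fires the combat start event, retargets the player camera, puts the player and active enemies into their combat states, and crossfades to combat audio.
; Each update, a timer that lengthens with enemy count tells all active enemies to engage offense.
; It switches to Victory when no enemies remain or Defeat when the player is dead.
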(event EventBeginPlay
  (|CallParentFunction) ; This node is disabled and will not be called.\nDrag off pins to build functionality.
)

(event EventTick
  (params (DeltaSeconds :type Float%20%28single-precision%29))
  (|CallParentFunction DeltaSeconds) ; This node is disabled and will not be called.\nDrag off pins to build functionality.
)

(fn OnStateEnter
  (bind _gamemanagerref (Variables|Default|GetGameManagerRef))
  (bind _gamemanagerref_2 (Variables|Default|GetGameManagerRef))
  (bind _playercamreference (Variables|/Game/OppositeGame/Systems/GameStates/BP_GameManager.BP_GameManager_C|GetPlayerCamReference _gamemanagerref))
  (bind _playerreference (Variables|/Game/OppositeGame/Systems/GameStates/BP_GameManager.BP_GameManager_C|GetPlayerReference _gamemanagerref))
  (|CallParentFunction)
  (Variables|Default|SetAttackTimer 0.0)
  (Default|CallCOMBATSTARTEVENT)
  (Default|SetCameraTarget _playercamreference (Variables|/Game/OppositeGame/BP_PlayerCamera.BP_PlayerCamera_C|GetTargetGame _playercamreference) false 0.0 "AC Combat Begin YEA")
  (Default|SwitchtoState _playerreference (Variables|/Game/OppositeGame/Systems/CharacterEntities/BP_CharacterBase.BP_CharacterBase_C|GetCombatStateToLoad _playerreference))
  (for _array_element (Variables|/Game/OppositeGame/Systems/GameStates/BP_GameManager.BP_GameManager_C|GetActiveEnemies (Variables|Default|GetGameManagerRef))
    (Default|SwitchtoState _array_element (Variables|/Game/OppositeGame/Systems/CharacterEntities/BP_CharacterBase.BP_CharacterBase_C|GetCombatStateToLoad _array_element)))
  (Audio|Components|Audio|FadeIn (Variables|/Game/OppositeGame/Systems/GameStates/BP_GameManager.BP_GameManager_C|GetAudioCombat _gamemanagerref_2) 2.0 1.0 0.0 "Linear" :!class /Script/Engine.AudioComponent)
  (Audio|Components|Audio|FadeOut (Variables|/Game/OppositeGame/Systems/GameStates/BP_GameManager.BP_GameManager_C|GetAudioCombatStart _gamemanagerref_2) 2.0 0.0 "Linear" :!class /Script/Engine.AudioComponent))

(fn OnStateUpdate
  (params (Deltatime :type Float%20%28double-precision%29))
  (bind _gamemanagerref (Variables|Default|GetGameManagerRef))
  (bind _gamemanagerref_2 (Variables|Default|GetGameManagerRef))
  (bind _gamemanagerref_3 (Variables|Default|GetGameManagerRef))
  (|CallParentFunction Deltatime)
  (Utilities|FlowControl|Sequence
    (:then_0
      (if (> (Utilities|Time|GetTimeSeconds) (Variables|Default|GetAttackTimer))
        (Variables|Default|SetAttackTimer (+ (+ (Variables|Default|GetAttackDelay) (Utilities|Time|GetTimeSeconds)) (* (Utilities|Array|Length (Variables|/Game/OppositeGame/Systems/GameStates/BP_GameManager.BP_GameManager_C|GetActiveEnemies _gamemanagerref)) (Variables|/Game/OppositeGame/Systems/GameStates/BP_GameManager.BP_GameManager_C|GetEnemyCountDelayMult _gamemanagerref))))
        (Development|PrintText "COMBAT TIMER TICK" true true "(R=1.000000,G=0.000000,B=0.000000,A=1.000000)")
        (for _array_element (Variables|/Game/OppositeGame/Systems/GameStates/BP_GameManager.BP_GameManager_C|GetActiveEnemies (Variables|Default|GetGameManagerRef))
          (Default|EngageOffense _array_element))))
    (:then_1
      (if (<= (Utilities|Array|Length (Variables|/Game/OppositeGame/Systems/GameStates/BP_GameManager.BP_GameManager_C|GetActiveEnemies (Variables|Default|GetGameManagerRef))) 0)
        (Default|SwitchtoState _gamemanagerref_3 (Variables|/Game/OppositeGame/Systems/GameStates/BP_GameManager.BP_GameManager_C|GetAC_Victory _gamemanagerref_3))))
    (:then_2
      (if (Variables|/Game/OppositeGame/Systems/CharacterEntities/BP_CharacterBase.BP_CharacterBase_C|GetIsDead (Variables|/Game/OppositeGame/Systems/GameStates/BP_GameManager.BP_GameManager_C|GetPlayerReference (Variables|Default|GetGameManagerRef)))
        (Default|SwitchtoState _gamemanagerref_2 (Variables|/Game/OppositeGame/Systems/GameStates/BP_GameManager.BP_GameManager_C|GetAC_Defeat _gamemanagerref_2))))))