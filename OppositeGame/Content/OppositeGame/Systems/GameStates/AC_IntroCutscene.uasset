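; Game state for the intro cutscene that puts the active enemies into their intro behavior.
; On entering, it loops over the game manager's active enemies and switches each one to the CST_Intro state.
; Its update only calls the parent, and it adds no exit logic of its own.
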(event EventBeginPlay
  (|CallParentFunction) ; This node is disabled and will not be called.\nDrag off pins to build functionality.
)

(event EventTick
  (params (DeltaSeconds :type Float%20%28single-precision%29))
  (|CallParentFunction DeltaSeconds) ; This node is disabled and will not be called.\nDrag off pins to build functionality.
)

(fn OnStateEnter
  (|CallParentFunction)
  (for _array_element (Variables|/Game/OppositeGame/Systems/GameStates/BP_GameManager.BP_GameManager_C|GetActiveEnemies (Variables|Default|GetGameManagerRef))
    (Default|SwitchtoState _array_element "/Game/OppositeGame/Systems/CharacterEntities/CST_Intro.CST_Intro_C")))

(fn OnStateUpdate
  (params (Deltatime :type Float%20%28double-precision%29))
  (|CallParentFunction Deltatime))