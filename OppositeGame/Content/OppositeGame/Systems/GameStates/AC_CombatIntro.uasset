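; Game-state component for the combat intro, run by the game manager before handing over to the combat state.
; On enter it plays the player's cinematic montage, times the state by the returned duration and sends active enemies walking to their combat start positions.
; Partway through it blends the camera to the game target.
; In the final fifth it interpolates enemies onto those positions, then switches to combat when the montage time ends.
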(event EventBeginPlay
  (|CallParentFunction) ; This node is disabled and will not be called.\nDrag off pins to build functionality.
)

(event EventTick
  (params (DeltaSeconds :type Float%20%28single-precision%29))
  (|CallParentFunction DeltaSeconds) ; This node is disabled and will not be called.\nDrag off pins to build functionality.
)

(fn OnStateEnter
  (bind _returnvalue (Utilities|Time|GetTimeSeconds))
  (bind _gamemanagerref (Variables|Default|GetGameManagerRef))
  (|CallParentFunction)
  (bind _montageduration (Default|PlayCinematicMontage (Variables|/Game/OppositeGame/Systems/GameStates/BP_GameManager.BP_GameManager_C|GetPlayerReference _gamemanagerref) (Variables|/Game/OppositeGame/Systems/GameStates/BP_GameManager.BP_GameManager_C|GetPlayerIntroMontag_Combat _gamemanagerref)))
  (Variables|Default|SetEndTime (+ _montageduration _returnvalue))
  (Variables|Default|SetLerpStartTimeSoDirty (+ _returnvalue (* _montageduration (Variables|/Game/OppositeGame/Systems/GameStates/BP_GameManager.BP_GameManager_C|GetIntroLerpStartTime (Variables|Default|GetGameManagerRef)))))
  (Variables|Default|SetFINALFLOATFIXTHEJERK _montageduration)
  (for _array_element (Variables|/Game/OppositeGame/Systems/GameStates/BP_GameManager.BP_GameManager_C|GetActiveEnemies _gamemanagerref)
    (AI|Navigation|SimpleMovetoLocation (Pawn|GetController _array_element) (Variables|/Game/OppositeGame/Systems/CharacterEntities/BP_CharacterBase.BP_CharacterBase_C|GetCombatStartTargetPosition _array_element))))

(fn OnStateUpdate
  (params (Deltatime :type Float%20%28double-precision%29))
  (bind _gamemanagerref (Variables|Default|GetGameManagerRef))
  (bind _gamemanagerref_2 (Variables|Default|GetGameManagerRef))
  (bind _playercamreference (Variables|/Game/OppositeGame/Systems/GameStates/BP_GameManager.BP_GameManager_C|GetPlayerCamReference _gamemanagerref))
  (|CallParentFunction Deltatime)
  (if (and (not (Variables|Default|GetMidstatelol)) (> (Utilities|Time|GetTimeSeconds) (Variables|Default|GetLerpStartTimeSoDirty)))
    (Variables|Default|SetMidstatelol true)
    (Default|SetCameraTarget _playercamreference (Variables|/Game/OppositeGame/BP_PlayerCamera.BP_PlayerCamera_C|GetTargetGame _playercamreference) true 1.0 "CombatIntro"))
  (if (> (Utilities|Time|GetTimeSeconds) (Variables|Default|GetEndTime))
    (Development|PrintText "SWITCHTOCOMBAT")
    (Default|SwitchtoState _gamemanagerref_2 (Variables|/Game/OppositeGame/Systems/GameStates/BP_GameManager.BP_GameManager_C|GetAC_Combat _gamemanagerref_2))
    (elif (> (Utilities|Time|GetTimeSeconds) (- (Variables|Default|GetEndTime) (* (Variables|Default|GetFINALFLOATFIXTHEJERK) 0.2)))
      (Development|PrintText "LERPFIX" true true "(R=0.094229,G=0.100249,B=1.000000,A=1.000000)")
      (for _array_element (Variables|/Game/OppositeGame/Systems/GameStates/BP_GameManager.BP_GameManager_C|GetActiveEnemies (Variables|Default|GetGameManagerRef))
        (Transformation|SetActorLocation _array_element (Math|Interpolation|VInterptoConstant (Transformation|GetActorLocation _array_element) (Math|Vector|MakeVector (.x (Variables|/Game/OppositeGame/Systems/CharacterEntities/BP_CharacterBase.BP_CharacterBase_C|GetCombatStartTargetPosition _array_element)) (.y (Variables|/Game/OppositeGame/Systems/CharacterEntities/BP_CharacterBase.BP_CharacterBase_C|GetCombatStartTargetPosition _array_element)) (Components|Capsule|GetScaledCapsuleHalfHeight (Variables|/Script/Engine.Character|GetCapsuleComponent _array_element))) Deltatime 1e+02) false false)))))