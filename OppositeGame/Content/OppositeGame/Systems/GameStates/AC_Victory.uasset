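; AC_Victory is the game state for winning a fight.
; On enter it switches the player to CST_WinState and fades out the combat audio through the game manager.
; Its update only calls the parent; the combat-start, attack-timer, enemy-engage and montage nodes are disconnected leftovers that never run.
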(event EventBeginPlay
  (|CallParentFunction) ; This node is disabled and will not be called.\nDrag off pins to build functionality.
)

(event EventTick
  (params (DeltaSeconds :type Float%20%28single-precision%29))
  (|CallParentFunction DeltaSeconds) ; This node is disabled and will not be called.\nDrag off pins to build functionality.
)

(fn OnStateEnter
  (bind _gamemanagerref (Variables|Default|GetGameManagerRef))
  (|CallParentFunction)
  (Default|SwitchtoState (Variables|/Game/OppositeGame/Systems/GameStates/BP_GameManager.BP_GameManager_C|GetPlayerReference _gamemanagerref) "/Game/OppositeGame/Systems/CharacterEntities/CST_WinState.CST_WinState_C")
  (Audio|Components|Audio|FadeOut (Variables|/Game/OppositeGame/Systems/GameStates/BP_GameManager.BP_GameManager_C|GetAudioCombat _gamemanagerref) 1.0 0.0 "Linear" :!class /Script/Engine.AudioComponent))

(fn OnStateUpdate
  (params (Deltatime :type Float%20%28double-precision%29))
  (|CallParentFunction Deltatime))