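; AC_Defeat is a game state component for defeat, sitting among the game's state systems.
; On enter, it uses the game manager reference to lerp the player camera to its Target0 and fade the combat audio out to silence.
; Update only calls the parent.
; The combat-start, attack-timer and enemy-engage nodes are disconnected and never run.
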(event EventBeginPlay
  (|CallParentFunction) ; This node is disabled and will not be called.\nDrag off pins to build functionality.
)

(event EventTick
  (params (DeltaSeconds :type Float%20%28single-precision%29))
  (|CallParentFunction DeltaSeconds) ; This node is disabled and will not be called.\nDrag off pins to build functionality.
)

(fn OnStateEnter
  (bind _gamemanagerref (Variables|Default|GetGameManagerRef))
  (bind _playercamreference (Variables|/Game/OppositeGame/Systems/GameStates/BP_GameManager.BP_GameManager_C|GetPlayerCamReference _gamemanagerref))
  (|CallParentFunction)
  (Default|SetCameraTarget _playercamreference (Variables|/Game/OppositeGame/BP_PlayerCamera.BP_PlayerCamera_C|GetTarget0 _playercamreference) true 0.5 "AC_Defeat")
  (Audio|Components|Audio|FadeOut (Variables|/Game/OppositeGame/Systems/GameStates/BP_GameManager.BP_GameManager_C|GetAudioCombat (Variables|Default|GetGameManagerRef)) 0.5 0.0 "Linear" :!class /Script/Engine.AudioComponent))

(fn OnStateUpdate
  (params (Deltatime :type Float%20%28double-precision%29))
  (|CallParentFunction Deltatime))